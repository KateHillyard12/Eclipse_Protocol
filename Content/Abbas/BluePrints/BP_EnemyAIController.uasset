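; Enemy AI controller that drives an enemy pawn toward the first player.
; On begin play, a looping timer repeatedly calls ChasePlayer, which on the server moves the pawn to player pawn 0 with a tight acceptance radius.
; A CanAttack flag only triggers a debug print, so no attack logic exists here.
; A branch targeting the second player is disconnected, and the gathered character list goes unused.
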(event Custom|ChasePlayer
  ;[0.15 0.15 0.15 0.5] Movement
  (Networking|SwitchHasAuthority
    (:Authority
      (Variables|Default|SetTargetActor (Game|Player|GetPlayerPawn 0))
      (Development|PrintString "moving")
      (Actor|GetAllActorsOfClass "/Script/Eclipse_Protocol.Eclipse_ProtocolCharacter")
      (AI|Navigation|MovetoActor self (Variables|Default|GetTargetActor) 1.0 true true true 0)
      (if (Variables|Default|GetcanAttack)
        (Development|PrintString "Attacking")))))

(event EventBeginPlay
  (Development|PrintString "Started")
  (Utilities|Time|SetTimerbyFunctionName 0 "ChasePlayer" 0.2 true))

(fn ConstructionScript)